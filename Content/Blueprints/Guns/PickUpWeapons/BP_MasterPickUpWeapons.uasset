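; Master Blueprint for weapon pickups that the player collects by interacting while inside a sphere trigger.
; Sphere overlap by an ALS character binds PickUP to that character's InteractObjects event and shows the pickup widget, both undone on overlap end.
; PickUP asks the player character cached at BeginPlay to spawn the configured weapon at its socket, then destroys the pickup if that succeeds.
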(event `self.ReceiveBeginPlay`
  (bind _asals_anim_man_character_bp (cast `/Game/AdvancedLocomotionV4/Blueprints/CharacterLogic/ALS_AnimMan_CharacterBP` (`GameplayStatics.GetPlayerCharacter` 0)))
  (set `self.CharacterRef` _asals_anim_man_character_bp))

(event `self.Sphere.OnComponentBeginOverlap`
  (params (OverlappedComponent :type "PrimitiveComponent Object Reference") (OtherActor :type "Actor Object Reference") (OtherComp :type "PrimitiveComponent Object Reference") (OtherBodyIndex :type Integer) (bFromSweep :type Boolean) (SweepResult :type "HitResult Structure (by ref)"))
  (bind _asals_anim_man_character_bp (cast `/Game/AdvancedLocomotionV4/Blueprints/CharacterLogic/ALS_AnimMan_CharacterBP` OtherActor))
  (add `/Game/AdvancedLocomotionV4/Blueprints/CharacterLogic/ALS_AnimMan_CharacterBP.InteractObjects` _asals_anim_man_character_bp (delegate `PickUP`))
  (`UserWidget.AddToViewport` (`/Game/AdvancedLocomotionV4/Blueprints/CharacterLogic/ALS_AnimMan_CharacterBP.WB_PickUpObjects` (`self.CharacterRef`)) 0))

(event `PickUP`
  (bind _sucess (`/Game/AdvancedLocomotionV4/Blueprints/CharacterLogic/ALS_AnimMan_CharacterBP.SpawnWeapons` (`self.CharacterRef`) (`self.Weapons`) (`self.WeaponSocket`)))
  (if _sucess
    (`self.K2_DestroyActor`)))

(event `self.Sphere.OnComponentEndOverlap`
  (params (OverlappedComponent :type "PrimitiveComponent Object Reference") (OtherActor :type "Actor Object Reference") (OtherComp :type "PrimitiveComponent Object Reference") (OtherBodyIndex :type Integer))
  (bind _asals_anim_man_character_bp (cast `/Game/AdvancedLocomotionV4/Blueprints/CharacterLogic/ALS_AnimMan_CharacterBP` OtherActor))
  (remove `/Game/AdvancedLocomotionV4/Blueprints/CharacterLogic/ALS_AnimMan_CharacterBP.InteractObjects` _asals_anim_man_character_bp (delegate `PickUP`))
  (`Widget.RemoveFromParent` (`/Game/AdvancedLocomotionV4/Blueprints/CharacterLogic/ALS_AnimMan_CharacterBP.WB_PickUpObjects` (`self.CharacterRef`))))

(fn `UserConstructionScript`)