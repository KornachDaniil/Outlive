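; Ammo pickup actor that gives the player character ammo for a configured weapon type and amount.
; Overlapping its collision binds the pickup to the character's InteractObjects dispatcher, and leaving unbinds it.
; On interact it calls AmmoPickUp on the player 0 character cached at BeginPlay, not the overlapping one, and destroys itself only if that call succeeds.
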(event `self.ReceiveBeginPlay`
  (bind _asals_anim_man_character_bp (cast `/Game/AdvancedLocomotionV4/Blueprints/CharacterLogic/ALS_AnimMan_CharacterBP` (`GameplayStatics.GetPlayerCharacter` 0)))
  (set `self.CharacterRef` _asals_anim_man_character_bp))

(event `self.PickUpCollision.OnComponentBeginOverlap`
  (params (OverlappedComponent :type "PrimitiveComponent Object Reference") (OtherActor :type "Actor Object Reference") (OtherComp :type "PrimitiveComponent Object Reference") (OtherBodyIndex :type Integer) (bFromSweep :type Boolean) (SweepResult :type "HitResult Structure (by ref)"))
  (bind _asals_anim_man_character_bp (cast `/Game/AdvancedLocomotionV4/Blueprints/CharacterLogic/ALS_AnimMan_CharacterBP` OtherActor))
  (add `/Game/AdvancedLocomotionV4/Blueprints/CharacterLogic/ALS_AnimMan_CharacterBP.InteractObjects` _asals_anim_man_character_bp (delegate `PickUpAmmo`)))

(event `PickUpAmmo`
  (bind _succses (`/Game/AdvancedLocomotionV4/Blueprints/CharacterLogic/ALS_AnimMan_CharacterBP.AmmoPickUp` (`self.CharacterRef`) (`self.Weapon`) (`self.AmmoCount`)))
  (if _succses
    (`self.K2_DestroyActor`)))

(event `self.PickUpCollision.OnComponentEndOverlap`
  (params (OverlappedComponent :type "PrimitiveComponent Object Reference") (OtherActor :type "Actor Object Reference") (OtherComp :type "PrimitiveComponent Object Reference") (OtherBodyIndex :type Integer))
  (bind _asals_anim_man_character_bp (cast `/Game/AdvancedLocomotionV4/Blueprints/CharacterLogic/ALS_AnimMan_CharacterBP` OtherActor))
  (remove `/Game/AdvancedLocomotionV4/Blueprints/CharacterLogic/ALS_AnimMan_CharacterBP.InteractObjects` _asals_anim_man_character_bp (delegate `PickUpAmmo`)))

(fn `UserConstructionScript`)